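; BP_Instance relays mission events to the text widget on the VR player's left hand.
; UpdateMission and FinalMission both cast player character 0 to BPC_VRPlayer, then get the BPC_LeftHandWidgetText from its LeftWidgetText component.
; Both events call that widget's UpdateMission, so FinalMission differs only in omitting the debug print.
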(event `self.UpdateMission`
  (`KismetSystemLibrary.PrintString` "Mission By Instance")
  (bind _asbpc_vrplayer (cast `/Game/2_BP/BPC_VRPlayer` (`GameplayStatics.GetPlayerCharacter` 0)))
  (bind _asbpc_left_hand_widget_text (cast `/Game/2_BP/Widget/BPC_LeftHandWidgetText` (`WidgetComponent.GetUserWidgetObject` (`VRPlayer.LeftWidget_Text` _asbpc_vrplayer))))
  (`/Game/2_BP/Widget/BPC_LeftHandWidgetText.UpdateMission` _asbpc_left_hand_widget_text))

(event `FinalMission`
  (bind _asbpc_vrplayer (cast `/Game/2_BP/BPC_VRPlayer` (`GameplayStatics.GetPlayerCharacter` 0)))
  (bind _asbpc_left_hand_widget_text (cast `/Game/2_BP/Widget/BPC_LeftHandWidgetText` (`WidgetComponent.GetUserWidgetObject` (`VRPlayer.LeftWidget_Text` _asbpc_vrplayer))))
  (`/Game/2_BP/Widget/BPC_LeftHandWidgetText.UpdateMission` _asbpc_left_hand_widget_text))