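; Base item Blueprint for objects that can be grabbed and released with a motion controller.
; Grab snaps the item to the controller's position and rotation, then reapplies the scale cached at BeginPlay.
; Release detaches it in place only if the releasing controller is the one currently holding it.
; An Active function returns false by default.
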(event `self.ReceiveBeginPlay`
  (set `self.OriginalScale` (`self.GetActorScale3D`)))

(event `/Game/2_BP/Legacy/GrabInterface.Grab`
  (params (MotionController :type "MotionControllerComponent Object Reference"))
  (bind _output_get (set `self.Motion Controller` MotionController))
  (`self.K2_AttachToComponent` _output_get "None" "SnapToTarget" "SnapToTarget" "KeepWorld")
  (`self.SetActorScale3D` (`self.OriginalScale`)))

(event `/Game/2_BP/Legacy/GrabInterface.Release`
  (params (MotionController :type "MotionControllerComponent Object Reference"))
  (if (== MotionController (`self.Motion Controller`))
    (set `self.Motion Controller` null)
    (`self.K2_DetachFromActor` "KeepWorld" "KeepWorld" "KeepWorld")))

(fn `Active`
  (returns (IsActive :type Boolean))
  (return false))

(fn `UserConstructionScript`)