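; BP_InventoryCase is a legacy Blueprint for an inventory case that holds four inventory components.
; BeginPlay turns off collision on all four components without changing their visibility.
; The CollisionEnable event restores query-and-physics collision and unhides the components in game, while CollisionDisable removes collision and hides them, toggling the case's contents as a group.
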(event `self.ReceiveBeginPlay`
  (`PrimitiveComponent.SetCollisionEnabled` (`self.InventoryComponent2`) "NoCollision")
  (`PrimitiveComponent.SetCollisionEnabled` (`self.InventoryComponent1`) "NoCollision")
  (`PrimitiveComponent.SetCollisionEnabled` (`self.InventoryComponent3`) "NoCollision")
  (`PrimitiveComponent.SetCollisionEnabled` (`self.InventoryComponent`) "NoCollision"))

(event `CollisionEnable`
  (bind _inventorycomponent1 (`self.InventoryComponent1`))
  (`PrimitiveComponent.SetCollisionEnabled` _inventorycomponent1 "QueryAndPhysics")
  (`PrimitiveComponent.SetCollisionEnabled` (`self.InventoryComponent3`) "QueryAndPhysics")
  (`PrimitiveComponent.SetCollisionEnabled` (`self.InventoryComponent2`) "QueryAndPhysics")
  (`PrimitiveComponent.SetCollisionEnabled` (`self.InventoryComponent`) "QueryAndPhysics")
  (`SceneComponent.SetHiddenInGame` _inventorycomponent1 false false)
  (`SceneComponent.SetHiddenInGame` (`self.InventoryComponent3`) false false)
  (`SceneComponent.SetHiddenInGame` (`self.InventoryComponent2`) false false)
  (`SceneComponent.SetHiddenInGame` (`self.InventoryComponent`) false false))

(event `CollisionDisable`
  (bind _inventorycomponent1 (`self.InventoryComponent1`))
  (`PrimitiveComponent.SetCollisionEnabled` _inventorycomponent1 "NoCollision")
  (`PrimitiveComponent.SetCollisionEnabled` (`self.InventoryComponent2`) "NoCollision")
  (`PrimitiveComponent.SetCollisionEnabled` (`self.InventoryComponent3`) "NoCollision")
  (`PrimitiveComponent.SetCollisionEnabled` (`self.InventoryComponent`) "NoCollision")
  (`SceneComponent.SetHiddenInGame` _inventorycomponent1 true false)
  (`SceneComponent.SetHiddenInGame` (`self.InventoryComponent2`) true false)
  (`SceneComponent.SetHiddenInGame` (`self.InventoryComponent`) true false)
  (`SceneComponent.SetHiddenInGame` (`self.InventoryComponent3`) true false))

(fn `UserConstructionScript`)