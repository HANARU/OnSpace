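; Legacy VR inventory slot component that snaps a released grabbable actor to itself.
; Begin overlap, with no valid GrabActor, filters for actors held by a controller other than ControllerToIgnore, but the GrabActor assignment shown is empty.
; End overlap clears GrabActor when that actor leaves.
; Tick attaches a valid GrabActor once its MotionController is invalid, keeping world scale; Active always returns false.
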(event `self.ReceiveBeginPlay`
  (add `self.OnComponentBeginOverlap` (delegate `BeginOverlap`))
  (add `self.OnComponentEndOverlap` (delegate `EndOverlap`)))

(event `BeginOverlap` :!signature `self.OnComponentBeginOverlap`
  (params (OverlappedComponent :type "PrimitiveComponent Object Reference") (OtherActor :type "Actor Object Reference") (OtherComp :type "PrimitiveComponent Object Reference") (OtherBodyIndex :type Integer) (bFromSweep :type Boolean) (SweepResult :type "HitResult Structure (by ref)"))
  (bind _controllertoignore (`self.ControllerToIgnore`))
  (`/Engine/EditorBlueprintResources/StandardMacros.IsValid` (`.GrabActor` (`self.GrabActor`))
    (:`Is Not Valid`
      (bind _asbp_item_base (cast `` OtherActor))
      (bind _motion_controller (`/Game/2_BP/Legacy/BP_InventoryComponent.Motion Controller` _asbp_item_base))
      (`/Engine/EditorBlueprintResources/StandardMacros.IsValid` _motion_controller
        (:`Is Valid`
          (`/Engine/EditorBlueprintResources/StandardMacros.IsValid` _controllertoignore
            (:`Is Valid`
              (if (!= _controllertoignore _motion_controller)
                (set `self.GrabActor` null _asbp_item_base :!label _label)))
            (:`Is Not Valid`
              (goto _label))))))))

(event `EndOverlap`
  (params (OverlappedComponent :type "PrimitiveComponent Object Reference") (OtherActor :type "Actor Object Reference") (OtherComp :type "PrimitiveComponent Object Reference") (OtherBodyIndex :type Integer))
  (if (== OtherActor (`.GrabActor` (`self.GrabActor`)))
    (set `self.GrabActor` null)))

(event `self.ReceiveTick`
  (params (DeltaSeconds :type "Float (single-precision)"))
  (bind (_grabactor _grabactor_2) (`self.GrabActor`))
  (`/Engine/EditorBlueprintResources/StandardMacros.IsValid` _grabactor_2
    (:`Is Valid`
      (`/Engine/EditorBlueprintResources/StandardMacros.IsValid` (`/Game/2_BP/Legacy/BP_InventoryComponent.Motion Controller` _grabactor_2)
        (:`Is Not Valid`
          (`Actor.K2_AttachToComponent` _grabactor_2 self "None" "SnapToTarget" "SnapToTarget" "KeepWorld" true))))))

(fn `Active`
  (returns (IsActive :type Boolean))
  (return false))