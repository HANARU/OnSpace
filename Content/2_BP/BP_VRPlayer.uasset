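; VR player Blueprint that passes head and hand tracking to its skeletal mesh's ABP_Player animation Blueprint.
; Each Tick casts the mesh's anim instance and writes world transforms from the camera as head input and from two arrow components as hand inputs.
; It also passes both motion controller transforms, crossed so the left controller fills the right variable and vice versa.
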(event `self.ReceiveTick`
  (params (DeltaSeconds :type "Float (single-precision)"))
  ;[1 1 1] Tick (send  val to ABP)
  (bind _asabp_player (cast `/Game/4_SK/VRPlayer/Anim/ABP_Player` (`SkeletalMeshComponent.GetAnimInstance` (`self.compSkeletal`))))
  (set `/Game/4_SK/VRPlayer/Anim/ABP_Player.In Head Transform World` (`SceneComponent.K2_GetComponentToWorld` (`self.compCam`)) _asabp_player)
  (set `/Game/4_SK/VRPlayer/Anim/ABP_Player.In Left Hand Transform World` (`SceneComponent.K2_GetComponentToWorld` (`self.ArrowLeft`)) _asabp_player)
  (set `/Game/4_SK/VRPlayer/Anim/ABP_Player.In Right Hand Transform World` (`SceneComponent.K2_GetComponentToWorld` (`self.ArrowRight`)) _asabp_player)
  (set `/Game/4_SK/VRPlayer/Anim/ABP_Player.RightControllerTransform` (`SceneComponent.K2_GetComponentToWorld` (`self.MotionControllerLeft`)) _asabp_player)
  (set `/Game/4_SK/VRPlayer/Anim/ABP_Player.LeftControllerTransform` (`SceneComponent.K2_GetComponentToWorld` (`self.MotionControllerRight`)) _asabp_player))

(fn `UserConstructionScript`)