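; BP_Navigator_Installed is the installation point for the Navigator item, whose delivery triggers the game-end event.
; On mesh overlap it casts the other actor to BPC_ItemBase and checks that ObjectName is "Navigator".
; A match destroys the item and swaps the mesh's three materials to show the installed device, then calls GameEnd.
; GameEnd currently only plays a 2D explosion sound.
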(event `self.StaticMeshComponent.OnComponentBeginOverlap`
  (params (OverlappedComponent :type "PrimitiveComponent Object Reference") (OtherActor :type "Actor Object Reference") (OtherComp :type "PrimitiveComponent Object Reference") (OtherBodyIndex :type Integer) (bFromSweep :type Boolean) (SweepResult :type "HitResult Structure (by ref)"))
  (bind _staticmeshcomponent (`self.StaticMeshComponent`))
  (bind _asbpc_item_base (cast `/Game/2_BP/BPC_ItemBase` OtherActor))
  (if (== (`ItemBase.objectName` _asbpc_item_base) "Navigator")
    (`self.K2_DestroyActor` _asbpc_item_base)
    (`PrimitiveComponent.SetMaterial` _staticmeshcomponent 0 "/Game/3_SM/CabinDoor/Mesh/MI_Base_Wall.MI_Base_Wall")
    (`PrimitiveComponent.SetMaterial` _staticmeshcomponent 1 "/Game/3_SM/Navigator/Mat/MI_Mesh_Decal.MI_Mesh_Decal")
    (`PrimitiveComponent.SetMaterial` _staticmeshcomponent 2 "/Game/3_SM/Navigator/Mat/MI_NormandyMonitor.MI_NormandyMonitor")
    (`self.Game End`)))

(event `Game End`
  (`GameplayStatics.PlaySound2D` "/Game/8_Sound/Explosion/Explosion_Big_02.Explosion_Big_02" 1.0 1.0 0.0 null null))

(fn `UserConstructionScript`)