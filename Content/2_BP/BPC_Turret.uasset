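; BPC_Turret is a turret that fires lasers and can be destroyed, leaving a wreck and an item actor.
; Shoot2Player waits briefly, then spawns a TurretLaser at the head's transform if the head still exists.
; DestroyAction plays an explosion, removes the head, swaps the body to a broken mesh, and spawns a BPC_ItemBase, calling its CallTurretDestroy.
; Neither event is triggered within this graph, and no aiming logic appears here.
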(event `self.Shoot2Player`
  (bind _turrethead (`self.TurretHead`))
  (bind (_returnvalue_location _returnvalue_rotation) (`KismetMathLibrary.BreakTransform` (`SceneComponent.K2_GetComponentToWorld` _turrethead)))
  (`KismetSystemLibrary.Delay` 2.0)
  (`/Engine/EditorBlueprintResources/StandardMacros.IsValid` _turrethead
    (:`Is Valid`
      (`|SpawnActorFromClass` "/Game/2_BP/TurretLaser.TurretLaser_C" (`KismetMathLibrary.MakeTransform` _returnvalue_location _returnvalue_rotation) "AlwaysSpawn" "MultiplyWithRoot" null null))))

(event `self.DestroyAction`
  (bind _turrethead (`self.TurretHead`))
  (`GameplayStatics.SpawnEmitterAtLocation` "/Game/5_FX/VFX/P_Explosion.P_Explosion" (`SceneComponent.K2_GetComponentLocation` _turrethead) (`SceneComponent.K2_GetComponentRotation` _turrethead) (10.0 10.0 10.0))
  (`ActorComponent.K2_DestroyComponent` (`self.TurretHead`))
  (`StaticMeshComponent.SetStaticMesh` (`self.TurretBody`) "/Game/3_SM/Turret/TurretBroken/SM_Broken_turret.SM_Broken_turret")
  (bind _returnvalue (`|SpawnActorFromClass` "/Game/2_BP/BPC_ItemBase.BPC_ItemBase_C" (`KismetMathLibrary.MakeTransform` (`SceneComponent.K2_GetComponentLocation` (`self.LaserStartPoint`))) "Undefined" "MultiplyWithRoot" null null))
  (`/Game/2_BP/BPC_ItemBase.TurretDestroy` _returnvalue))

(fn `UserConstructionScript`)