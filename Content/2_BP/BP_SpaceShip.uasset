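; Spaceship actor with sliding interior and exterior doors that open for the VR character, plus zones that switch it between flying outside and walking inside.
; Fly and Walk collision overlaps set the character's movement mode.
; Each door's trigger plays sounds and a Timeline driving absolute world Y, guarded by DoOnce until finished; opening either door also sets OxygenActivate true.
; The DoorMove function is an unfinished stub, and the cached initial door locations are unused.
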(event `self.ReceiveBeginPlay`
  (set `self.ExteriorDoorFirtstLoc` (`SceneComponent.K2_GetComponentLocation` (`self.ExteriorDoor`)))
  (set `self.InteriorDoorFirstLoc` (`SceneComponent.K2_GetComponentLocation` (`self.InteriorDoor`)))
  (bind _asvrcharacter (cast `/Game/2_BP/VRCharacter` (`GameplayStatics.GetPlayerCharacter` 0)))
  (set `self.Player` _asvrcharacter))

(event `self.FlyCollision.OnComponentBeginOverlap`
  (params (OverlappedComponent :type "PrimitiveComponent Object Reference") (OtherActor :type "Actor Object Reference") (OtherComp :type "PrimitiveComponent Object Reference") (OtherBodyIndex :type Integer) (bFromSweep :type Boolean) (SweepResult :type "HitResult Structure (by ref)"))
  ;[1 1 1] OutDoor Fly Condition
  (bind _asvrcharacter (cast `/Game/2_BP/VRCharacter` OtherActor))
  (`/Engine/EditorBlueprintResources/StandardMacros.IsValid` _asvrcharacter
    (:`Is Valid`
      (bind _charactermovement (`Character.CharacterMovement` _asvrcharacter))
      (if (`CharacterMovementComponent.IsWalking` _charactermovement)
        (`CharacterMovementComponent.SetMovementMode` _charactermovement "MOVE_Flying" 0)
        (`KismetSystemLibrary.PrintString` "Fly")))))

(event `self.WalkCollision.OnComponentBeginOverlap`
  (params (OverlappedComponent :type "PrimitiveComponent Object Reference") (OtherActor :type "Actor Object Reference") (OtherComp :type "PrimitiveComponent Object Reference") (OtherBodyIndex :type Integer) (bFromSweep :type Boolean) (SweepResult :type "HitResult Structure (by ref)"))
  ;[1 1 1] InDoor Walk Condition
  (bind _asvrcharacter (cast `/Game/2_BP/VRCharacter` OtherActor))
  (`/Engine/EditorBlueprintResources/StandardMacros.IsValid` _asvrcharacter
    (:`Is Valid`
      (bind _charactermovement (`Character.CharacterMovement` _asvrcharacter))
      (if (`NavMovementComponent.IsFlying` _charactermovement)
        (`CharacterMovementComponent.SetMovementMode` _charactermovement "MOVE_Walking" 0)
        (`KismetSystemLibrary.PrintString` "Walk")))))

(event `self.IndoorCollision.OnComponentBeginOverlap`
  (params (OverlappedComponent :type "PrimitiveComponent Object Reference") (OtherActor :type "Actor Object Reference") (OtherComp :type "PrimitiveComponent Object Reference") (OtherBodyIndex :type Integer) (bFromSweep :type Boolean) (SweepResult :type "HitResult Structure (by ref)"))
  (bind _interiordoor (`self.InteriorDoor`))
  (bind (_returnvalue_x _returnvalue_y _returnvalue_z) (`KismetMathLibrary.BreakVector` (`SceneComponent.K2_GetComponentLocation` _interiordoor)))
  ;[1 0.3031 0.3031] InDoor
  ;;[1 1 1] Open InDoor
  (bind _asvrcharacter (cast `/Game/2_BP/VRCharacter` OtherActor))
  (`/Engine/EditorBlueprintResources/StandardMacros.IsValid` _asvrcharacter
    (:`Is Valid`
      (`/Engine/EditorBlueprintResources/StandardMacros.DoOnce` false :!label _label
        (:`Completed`
          (set `/Game/2_BP/VRCharacter.OxygenActivate` true _asvrcharacter)
          (`GameplayStatics.PlaySound2D` "/Game/8_Sound/Door/S_Door_Open_03.S_Door_Open_03" 1.0 1.0 0.0 null null)
          (`GameplayStatics.PlaySound2D` "/Game/8_Sound/Door/S_Door_Open_04.S_Door_Open_04" 1.0 1.0 0.0 null null)
          (bind (_direction _doormove) (`Timeline|Timeline` :!via `PlayFromStart`)
            (:`Update`
              (`SceneComponent.K2_SetWorldLocation` _interiordoor (`KismetMathLibrary.MakeVector` _returnvalue_x _doormove _returnvalue_z) false false))
            (:`Finished`
              (goto _label :!via `Reset`))))))))

(event `self.IndoorCollision.OnComponentEndOverlap`
  (params (OverlappedComponent :type "PrimitiveComponent Object Reference") (OtherActor :type "Actor Object Reference") (OtherComp :type "PrimitiveComponent Object Reference") (OtherBodyIndex :type Integer))
  (bind _interiordoor (`self.InteriorDoor`))
  (bind (_returnvalue_x _returnvalue_y _returnvalue_z) (`KismetMathLibrary.BreakVector` (`SceneComponent.K2_GetComponentLocation` _interiordoor)))
  ;[1 0.3031 0.3031] InDoor
  ;;[1 1 1] Close InDoor
  (bind _asvrcharacter (cast `/Game/2_BP/VRCharacter` OtherActor))
  (`/Engine/EditorBlueprintResources/StandardMacros.IsValid` _asvrcharacter
    (:`Is Valid`
      (`/Engine/EditorBlueprintResources/StandardMacros.DoOnce` false :!label _label_2
        (:`Completed`
          (`GameplayStatics.PlaySound2D` "/Game/8_Sound/Door/S_Door_Close_03.S_Door_Close_03" 1.0 1.0 0.0 null null)
          (bind (_direction _doormove) (`Timeline|Timeline_0` :!via `ReverseFromEnd`)
            (:`Update`
              (`SceneComponent.K2_SetWorldLocation` _interiordoor (`KismetMathLibrary.MakeVector` _returnvalue_x _doormove _returnvalue_z) false false))
            (:`Finished`
              (goto _label_2 :!via `Reset`))))))))

(event `self.OutdoorCollision.OnComponentBeginOverlap`
  (params (OverlappedComponent :type "PrimitiveComponent Object Reference") (OtherActor :type "Actor Object Reference") (OtherComp :type "PrimitiveComponent Object Reference") (OtherBodyIndex :type Integer) (bFromSweep :type Boolean) (SweepResult :type "HitResult Structure (by ref)"))
  (bind _exteriordoor (`self.ExteriorDoor`))
  (bind (_returnvalue_x _returnvalue_y _returnvalue_z) (`KismetMathLibrary.BreakVector` (`SceneComponent.K2_GetComponentLocation` _exteriordoor)))
  ;[0 0.1333 1] OutDoor
  ;;[1 1 1] Open OutDoor
  (bind _asvrcharacter (cast `/Game/2_BP/VRCharacter` OtherActor))
  (`/Engine/EditorBlueprintResources/StandardMacros.IsValid` _asvrcharacter
    (:`Is Valid`
      (`/Engine/EditorBlueprintResources/StandardMacros.DoOnce` false :!label _label_3
        (:`Completed`
          (set `/Game/2_BP/VRCharacter.OxygenActivate` true _asvrcharacter)
          (`GameplayStatics.PlaySound2D` "/Game/8_Sound/Door/S_Door_Open_03.S_Door_Open_03" 1.0 1.0 0.0 null null)
          (`GameplayStatics.PlaySound2D` "/Game/8_Sound/Door/S_Door_Open_04.S_Door_Open_04" 1.0 1.0 0.0 null null)
          (bind (_direction _doormove) (`Timeline|Timeline_1` :!via `PlayFromStart`)
            (:`Update`
              (`SceneComponent.K2_SetWorldLocation` _exteriordoor (`KismetMathLibrary.MakeVector` _returnvalue_x _doormove _returnvalue_z) false false))
            (:`Finished`
              (goto _label_3 :!via `Reset`))))))))

(event `self.OutdoorCollision.OnComponentEndOverlap`
  (params (OverlappedComponent :type "PrimitiveComponent Object Reference") (OtherActor :type "Actor Object Reference") (OtherComp :type "PrimitiveComponent Object Reference") (OtherBodyIndex :type Integer))
  (bind _exteriordoor (`self.ExteriorDoor`))
  (bind (_returnvalue_x _returnvalue_y _returnvalue_z) (`KismetMathLibrary.BreakVector` (`SceneComponent.K2_GetComponentLocation` _exteriordoor)))
  ;[0 0.1333 1] OutDoor
  ;;[1 1 1] Close OutDoor
  (bind _asvrcharacter (cast `/Game/2_BP/VRCharacter` OtherActor))
  (`/Engine/EditorBlueprintResources/StandardMacros.IsValid` _asvrcharacter
    (:`Is Valid`
      (`/Engine/EditorBlueprintResources/StandardMacros.DoOnce` false :!label _label_4
        (:`Completed`
          (`GameplayStatics.PlaySound2D` "/Game/8_Sound/Door/S_Door_Close_03.S_Door_Close_03" 1.0 1.0 0.0 null null)
          (bind (_direction _doormove) (`Timeline|Timeline_2` :!via `ReverseFromEnd`)
            (:`Update`
              (`SceneComponent.K2_SetWorldLocation` _exteriordoor (`KismetMathLibrary.MakeVector` _returnvalue_x _doormove _returnvalue_z) false false))
            (:`Finished`
              (goto _label_4 :!via `Reset`))))))))

(fn `Door Move`
  (params (Door :type "StaticMeshComponent Object Reference") (Close :type Boolean))
  (locals (DoorObj :type "StaticMeshComponent Object Reference"))
  (set `local.DoorObj` Door)
  (if Close
    _))

(fn `UserConstructionScript`)